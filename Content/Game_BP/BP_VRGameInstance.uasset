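; VR game instance that decides at startup whether the game runs in VR or flat-screen mode.
; On Init it sets IsFlatmode to false only when a head-mounted display is both connected and enabled, and always switches ShowDeveloperCode on.
; Two getter functions expose these flags.
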(event `self.ReceiveInit`
  (`|ExecutionSequence`
    (:`then_0`
      (set `self.Show_developer_code?` true))
    (:`then_1`
      (if (and (`HeadMountedDisplayFunctionLibrary.IsHeadMountedDisplayConnected`) (`HeadMountedDisplayFunctionLibrary.IsHeadMountedDisplayEnabled`))
        (set `self.Is_flatmode?` false)
        (else
          (set `self.Is_flatmode?` true))))))

(fn `IsFlatmode`
  (returns (`IsFlatmode?` :type Boolean))
  (return (`self.Is_flatmode?`)))

(fn `ShowDeveloperCode`
  (returns (ShowDeveloperCode :type Boolean))
  (return (`self.Show_developer_code?`)))