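; Restaurant game mode that runs the order loop: random recipe orders on a screen widget, an NPC customer and a food tray.
; Init indexes recipes by exact tag-set key and by anchor tags.
; Ringing the bell matches tray items' gameplay tags to orders through the exact-key map, only for recipes disallowing extra ingredients.
; Orders are marked correct or wrong; full success sends the customer out and starts new orders.
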(event `self.ReceiveBeginPlay`
  ;[0.01591 0.15 0 0.5] Initilize
  (`self.Init`)
  (bind _returnvalue (`GameplayStatics.GetActorOfClass` "/Game/AI/BP_Simple_NPC_AI.BP_Simple_NPC_AI_C"))
  (set `self.SimpleAi_Ref` _returnvalue)
  (`KismetSystemLibrary.Delay` 2.0)
  (`self.Handle start order`))

(event `Clear orders`
  (`KismetArrayLibrary.Array_Clear` (`self.CurentOrders`))
  (`KismetArrayLibrary.Array_Clear` (`self.RecivedOrders`))
  (set `self.MaxOrderAmount` 0)
  (message `/Game/Blueprints/BPI/BPI_Widget.Clear all` (`self.W_OrderScreenRef`)))

(event `/Game/Blueprints/BPI/BPI_GameMode.DebugTest`
  ;[0.15 0.00341 0 0.5] Remove later
  ;[0.06452 0.15 0.06564 0.5] Handle start order
  (`self.Clear orders` :!label _label)
  (`/Game/Blueprints/BPFL/BPFL_GlobalFunctions.Debug - Print string` "START ORDER" true (struct :`R` 1.0 :`G` 0.715079 :`A` 1.0))
  (set `self.MaxOrderAmount` 4)
  (`self.HandleStartOrder`)
  (`/Game/AI/BP_Simple_NPC_AI.Walk to counter` (`self.SimpleAi_Ref`))
  (`KismetSystemLibrary.Delay` 3.0)
  (`SceneComponent.SetVisibility` (`/Game/Blueprints/GamePlay/BP_FoodTray.StaticMesh` (`self.FoodTrayRef`)) true false))

(event `Handle start order`
  (goto _label))

(event `/Game/Blueprints/BPI/BPI_GameMode.RingBtnPressed`
  (if (not (== (`KismetArrayLibrary.Array_Length` (`self.CurentOrders`)) 0)) :!label _label_2
    ;[0.06399 0.4635 0 0.5] Complete Order Info Check
    (`/Game/Blueprints/BPFL/BPFL_GlobalFunctions.Debug - Print string` "CHECKING ORDER..." true (struct :`R` 1.0 :`G` 0.715079 :`A` 1.0))
    (`KismetArrayLibrary.Array_Clear` (`self.RecivedOrders`))
    (bind _foodorder (message `/Game/Blueprints/BPI/BPI_GameMode.HandleReciveFood` (`self.FoodTrayRef`)))
    (for _array_element _foodorder
      (`|ExecutionSequence`
        (:`then_0`
          (`/Game/Blueprints/BPFL/BPFL_GlobalFunctions.Debug - Print string` (`KismetSystemLibrary.GetDisplayName` _array_element) false))
        (:`then_1`
          (bind _tags (message `/Game/Blueprints/BPI/BPI_GameMode.Recive item recipe Tags` _array_element))
          (`KismetArrayLibrary.Array_Add` (`self.RecivedOrders`) _tags))))
    (`/Game/Blueprints/BPFL/BPFL_GlobalFunctions.Debug - GameplayTagContainer` (struct) (`self.RecivedOrders`) false)
    (`self.ExamineOrder`)))

(event `/Game/Blueprints/BPI/BPI_GameMode.DebugTestRingBell`
  ;[0.15 0.00341 0 0.5] Remove later
  (goto _label_2))

(event `HandleStartOrder`
  ;[0.4167 0.128 0 0.5] HandleStartOrder
  (for _index (range (`self.MaxOrderAmount`))
    (`KismetArrayLibrary.Array_Set` (`self.CurentOrders`) _index (make `/Game/Blueprints/Structs/ST_Order` _index (`KismetArrayLibrary.Array_Random` (`self.AllRecipe`))) true))
  (message `/Game/Blueprints/BPI/BPI_GameMode.HandleOrderTask` (`self.W_OrderScreenRef`) (`self.CurentOrders`)))

(event `ExamineOrder`
  (bind (_recipe_ref_index _recipe_ref_recipe) (break `/Game/Blueprints/Structs/ST_Order` (`self.Recipe Ref`)))
  (bind (_recipe_ref_index_2 _recipe_ref_recipe_2) (break `/Game/Blueprints/Structs/ST_Order` (`self.Recipe Ref`)))
  (bind (_output_index _output_recipe) (break `/Game/Blueprints/Structs/ST_Order` (`|GetArrayItem` (`self.CurentOrders`) (`self.Recipe index ref`))))
  (bind (_output_index_2 _output_recipe_2) (break `/Game/Blueprints/Structs/ST_Order` (`|GetArrayItem` (`self.CurentOrders`) (`self.Recipe index ref`))))
  (bind (_output_index_3 _output_recipe_3 _output_status) (break `/Game/Blueprints/Structs/ST_Order` (`|GetArrayItem` (`self.CurentOrders`) (- (`self.MaxOrderAmount`) 1))))
  (set `self.Wrong order count` 0)
  (for (_array_element _array_index) (`self.CurentOrders`)
    (set `self.Recipe Ref` _array_element)
    (set `self.Recipe index ref` _array_index)
    ;[0.6042 0.2025 0 0.5] Comment
    (if (not (`/Game/Blueprints/DataAssets/Recipes/DA_Recipe.AllowExtraIngredients` _recipe_ref_recipe_2))
      ;[0.003585 0.15 0 0.5] Comment
      (if (> (`KismetArrayLibrary.Array_Length` (`self.RecivedOrders`)) 0)
        (for (_array_element_2 _array_index_2) (`self.RecivedOrders`)
          (bind _tagkeys (`/Game/Blueprints/BPFL/BPFL_GlobalFunctions.MakeTagKey(Tags: GameplayTagContainer) → String` _array_element_2))
          (bind (_value _returnvalue) (`BlueprintMapLibrary.Map_Find` (`self.ExactKeyToRecipe`) _tagkeys))
          (if (and _returnvalue (== _value _recipe_ref_recipe))
            (`KismetArrayLibrary.Array_Set` (`self.CurentOrders`) (`self.Recipe index ref`) (make `/Game/Blueprints/Structs/ST_Order` _output_index_2 _output_recipe_2 "NewEnumerator1"))
            (`KismetArrayLibrary.Array_Remove` (`self.RecivedOrders`) _array_index_2)
            (set `self.FoundOrder?` true)
            (break)))
        (if (`self.FoundOrder?`)
          (set `self.FoundOrder?` false)
          (else
            (set `self.Wrong order count` (+ (`self.Wrong order count`) 1) :!label _label_3)
            (`KismetArrayLibrary.Array_Set` (`self.CurentOrders`) (`self.Recipe index ref`) (make `/Game/Blueprints/Structs/ST_Order` _output_index _output_recipe "NewEnumerator2"))))
        (else
          (goto _label_3)))))
  (if (select `/Game/Blueprints/Enums/E_OrderStatus` _output_status :`NewEnumerator1` true :`NewEnumerator2` true)
    (if (> (`self.Wrong order count`) 0)
      (`self.Order failed`)
      (else
        (`self.Order completed`)))))

(event `Order completed`
  (bind _foodtrayref (`self.FoodTrayRef`))
  (`/Game/Blueprints/BPFL/BPFL_GlobalFunctions.Debug - Print string` "ORDER COMPLETED" true (struct :`R` 0.038153 :`G` 1.0 :`A` 1.0))
  (`self.Update order status`)
  (`|ExecutionSequence`
    (:`then_0`
      (`self.Print order status` true)
      (`/Game/AI/BP_Simple_NPC_AI.Move from counter to exit` (`self.SimpleAi_Ref`))
      (`/Game/Blueprints/BPI/BPI_GameMode.Clear` _foodtrayref)
      (`SceneComponent.SetVisibility` (`/Game/Blueprints/GamePlay/BP_FoodTray.StaticMesh` _foodtrayref) false false))
    (:`then_1`
      (`KismetSystemLibrary.Delay` 3.0)
      (`self.Handle start order`))))

(event `Order failed`
  (`/Game/Blueprints/BPFL/BPFL_GlobalFunctions.Debug - Print string` "ORDER FAILED" true (struct :`R` 1.0 :`B` 0.025124 :`A` 1.0))
  (`self.Update order status`)
  (`self.Print order status` true))

(event `Update order status`
  (`/Game/Blueprints/BPI/BPI_GameMode.W - Highlight order status` (`self.W_OrderScreenRef`) (`self.CurentOrders`)))

(fn `GetWidget`
  (returns (widgetRef :type "/Game/Widgets/TV_Widgets/W_MainOrderScreen Object Reference"))
  (return (`self.W_OrderScreenRef`)))

(fn `HandleReciveFood`)

(fn `Init`
  (`|ExecutionSequence`
    (:`then_0`)
    (:`then_1`
      (bind _returnvalue (`|CreateWidget` "/Game/Widgets/TV_Widgets/W_MainOrderScreen.W_MainOrderScreen_C"))
      (set `self.W_OrderScreenRef` _returnvalue)
      (bind _returnvalue_2 (`GameplayStatics.GetActorOfClass` "/Game/Blueprints/GamePlay/BP_FoodTray.BP_FoodTray_C"))
      (bind _output_get (set `self.FoodTrayRef` _returnvalue_2))
      (`SceneComponent.SetVisibility` (`/Game/Blueprints/GamePlay/BP_FoodTray.StaticMesh` _output_get) false false))
    (:`then_2`
      ;[0 0.15 0.004348 0.5] ExactKeyToRecipe
      (for _array_element (`self.AllRecipe`)
        (bind _tagkeys (`/Game/Blueprints/BPFL/BPFL_GlobalFunctions.MakeTagKey(Tags: GameplayTagContainer) → String` (`/Game/Blueprints/DataAssets/Recipes/DA_Recipe.RequiredTags` _array_element)))
        (`BlueprintMapLibrary.Map_Add` (`self.ExactKeyToRecipe`) _tagkeys _array_element)))
    (:`then_3`
      ;[0.1667 0.07716 0 0.5] Anchor index
      (for _array_element_2 (`self.AllRecipe`)
        (`self.Make anchor Index` _array_element_2))
      (if (`/Game/Blueprints/BPFL/BPFL_GlobalFunctions.ShowDeveloperCode`)
        (`/Game/Blueprints/BPFL/BPFL_GlobalFunctions.Debug - ST_AnchorIndex` (`self.AnchorIndex`))))))

(fn `IsTool`
  (returns (IsTool :type Boolean))
  (return false))

(fn `Make anchor Index`
  (params (Recipe :type "/Game/Blueprints/DataAssets/Recipes/DA_Recipe Object Reference"))
  (locals (`L-Recipe` :type "/Game/Blueprints/DataAssets/Recipes/DA_Recipe Object Reference") (`?wasFound` :type Boolean))
  (set `local.L-Recipe` Recipe)
  (for _array_element (`BlueprintGameplayTagLibrary.BreakGameplayTagContainer` (`/Game/Blueprints/DataAssets/Recipes/DA_Recipe.AnchorTags` Recipe))
    (for (_array_element_2 _array_index) (`self.AnchorIndex`)
      (if (`BlueprintGameplayTagLibrary.MatchesTag` (`.index_8_18BAC2404E8D79289E7B83A70D7E2831` (break `/Game/Blueprints/Structs/ST_AnchorIndex` _array_element_2)) _array_element true)
        (`KismetArrayLibrary.Array_AddUnique` (`.AllRecipesValue_6_73BC53D748ABD1924AD82C80170958ED` (break `/Game/Blueprints/Structs/ST_AnchorIndex` (`|GetArrayItem` (`self.AnchorIndex`) _array_index))) (`local.L-Recipe`))
        (set `local.?wasFound` true)
        (break)))
    (if (`local.?wasFound`)
      (set `local.?wasFound` false)
      (else
        (bind _returnvalue (`KismetArrayLibrary.Array_Add` (`self.AnchorIndex`) (make `/Game/Blueprints/Structs/ST_AnchorIndex` _array_element)))
        (`KismetArrayLibrary.Array_AddUnique` (`.AllRecipesValue_6_73BC53D748ABD1924AD82C80170958ED` (break `/Game/Blueprints/Structs/ST_AnchorIndex` (`|GetArrayItem` (`self.AnchorIndex`) _returnvalue))) (`local.L-Recipe`))))))

(fn `Print order status`
  (params (bPrintToScreen :type Boolean))
  (if (`/Game/Blueprints/BPFL/BPFL_GlobalFunctions.ShowDeveloperCode`)
    (for _array_element (`self.CurentOrders`)
      (switch `/Game/Blueprints/Enums/E_OrderStatus` (`.Status_8_491CE6594C35E2A5099687B79BE97CC6` (break `/Game/Blueprints/Structs/ST_Order` _array_element))
        (:`NewEnumerator1`
          (`/Game/Blueprints/BPFL/BPFL_GlobalFunctions.Debug - Print string` (`KismetTextLibrary.Conv_TextToString` (`|FormatText` "CORRECT ORDER: {!}" (`.Recipe_7_00323842465D3AB69D91A590D369E653` (break `/Game/Blueprints/Structs/ST_Order` _array_element)))) bPrintToScreen (struct :`R` 0.042388 :`G` 1.0 :`A` 1.0)))
        (:`NewEnumerator2`
          (`/Game/Blueprints/BPFL/BPFL_GlobalFunctions.Debug - Print string` (`KismetTextLibrary.Conv_TextToString` (`|FormatText` "WRONG ORDER: {!}" (`.Recipe_7_00323842465D3AB69D91A590D369E653` (break `/Game/Blueprints/Structs/ST_Order` _array_element)))) bPrintToScreen (struct :`R` 1.0 :`B` 0.008842 :`A` 1.0)))))))

(fn `Recive item recipe Tags`
  (returns (Tags :type "GameplayTagContainer Structure"))
  (return))

(fn `rest`
  (params (Array :type "Array of /Game/Blueprints/Structs/ST_Order Structure") (TextColor :type "LinearColor Structure"))
  (for _array_element Array
    (`/Game/Blueprints/BPFL/BPFL_GlobalFunctions.Debug - Print string` (`|GetEnumeratorNameAsString` (`.Status_8_491CE6594C35E2A5099687B79BE97CC6` (break `/Game/Blueprints/Structs/ST_Order` _array_element))) true TextColor)))

(fn `UserConstructionScript`)