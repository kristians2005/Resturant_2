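; Simple NPC actor that moves its NPC component along splines, with one route from start to counter and another from counter to exit.
; Two custom events each play a timeline at a rate of 1/Speed, so a higher Speed means a slower walk.
; Timeline alpha maps to distance along the referenced spline, setting world location and rotation.
; BeginPlay and Tick are empty; an older per-frame spline movement is left disconnected.
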(event `self.ReceiveBeginPlay`)

(event `self.ReceiveTick`
  (params (DeltaSeconds :type "Float (single-precision)")))

(event `Walk to counter`
  (bind _spline (`/Game/AI/BP_Spline.Spline` (`self.start-to-counter_Spline`)))
  (`TimelineComponent.SetPlayRate` (`self.WalkToCounter`) (/ 1.0 (`self.Speed`)))
  (bind (_direction _alpha) (`Timeline|WalkToCounter` :!via `PlayFromStart`)
    (:`Update`
      (bind _returnvalue (`KismetMathLibrary.Lerp` 0.0 (`SplineComponent.GetSplineLength` (`/Game/AI/BP_Spline.Spline` (`self.start-to-counter_Spline`))) _alpha))
      (bind (_returnvalue_roll _returnvalue_pitch _returnvalue_yaw) (`KismetMathLibrary.BreakRotator` (`SplineComponent.GetRotationAtDistanceAlongSpline` _spline _returnvalue "World")))
      (`SceneComponent.K2_SetWorldLocationAndRotation` (`self.NPC`) (`SplineComponent.GetLocationAtDistanceAlongSpline` _spline _returnvalue "World") (`KismetMathLibrary.MakeRotator` _returnvalue_roll _returnvalue_pitch _returnvalue_yaw) false false))))

(event `Move from counter to exit`
  (bind _spline (`/Game/AI/BP_Spline.Spline` (`self.counter-to-exit_spline`)))
  (`TimelineComponent.SetPlayRate` (`self.Countertoexit`) (/ 1.0 (`self.Speed`)))
  (bind (_direction _alpha) (`Timeline|Countertoexit` :!via `PlayFromStart`)
    (:`Update`
      (bind _returnvalue (`KismetMathLibrary.Lerp` 0.0 (`SplineComponent.GetSplineLength` (`/Game/AI/BP_Spline.Spline` (`self.counter-to-exit_spline`))) _alpha))
      (bind (_returnvalue_roll _returnvalue_pitch _returnvalue_yaw) (`KismetMathLibrary.BreakRotator` (`SplineComponent.GetRotationAtDistanceAlongSpline` _spline _returnvalue "World")))
      (`SceneComponent.K2_SetWorldLocationAndRotation` (`self.NPC`) (`SplineComponent.GetLocationAtDistanceAlongSpline` _spline _returnvalue "World") (`KismetMathLibrary.MakeRotator` _returnvalue_roll _returnvalue_pitch _returnvalue_yaw) false false))))

(fn `UserConstructionScript`)