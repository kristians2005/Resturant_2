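; BP_OrderPaper is an order paper Blueprint that holds a FoodOrder collection for the gameplay's food order handling.
; HandleReciveFood returns FoodOrder when it is non-empty, and FlatMode_Interaction reports a fixed interaction type.
; The recipe tag and widget getters are empty stubs, and the event graph and construction script contain no logic.
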(event `self.ReceiveBeginPlay`)

(fn `FlatMode_Interaction`
  (returns (BaseItemMasterRef :type "/Game/Blueprints/CookingItems/A_BP_BaseItem_Master Object Reference") (InteractionType :type "/Game/Blueprints/Enums/E_InteractionTypes Enum") (Actor :type "Actor Object Reference"))
  (return null "NewEnumerator0" null))

(fn `GetWidget`
  (returns (widgetRef :type "/Game/Widgets/TV_Widgets/W_MainOrderScreen Object Reference"))
  (return null))

(fn `HandleReciveFood`
  (returns (FoodOrder :type "Array of Actor Object Reference"))
  (if (> (`KismetArrayLibrary.Array_Length` (`self.FoodOrder`)) 0)
    (return (`self.FoodOrder`))))

(fn `Recive item recipe Tags`
  (returns (Tags :type "GameplayTagContainer Structure"))
  (return))

(fn `UserConstructionScript`)