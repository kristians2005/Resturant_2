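; BP_FoodTray is a tray actor that tracks which food items are placed on it as a food order.
; Overlaps on its collision component add or remove actors tagged "food" in FoodOrder, counting only their "BaseItemCol" components.
; HandleReciveFood returns that array when non-empty.
; Clear destroys every item and empties the array, switching off end-overlap removal meanwhile so the array stays intact during the loop.
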(event `self.ReceiveBeginPlay`)

(event `self.HandleFoodOrderCollision.OnComponentBeginOverlap`
  (params (OverlappedComponent :type "PrimitiveComponent Object Reference") (OtherActor :type "Actor Object Reference") (OtherComp :type "PrimitiveComponent Object Reference") (OtherBodyIndex :type Integer) (bFromSweep :type Boolean) (SweepResult :type "HitResult Structure (by ref)"))
  (if (and (`self.ActorHasTag` OtherActor "food") (`ActorComponent.ComponentHasTag` OtherComp "BaseItemCol"))
    (`KismetArrayLibrary.Array_Add` (`self.FoodOrder`) OtherActor)))

(event `self.HandleFoodOrderCollision.OnComponentEndOverlap`
  (params (OverlappedComponent :type "PrimitiveComponent Object Reference") (OtherActor :type "Actor Object Reference") (OtherComp :type "PrimitiveComponent Object Reference") (OtherBodyIndex :type Integer))
  (bind _foodorder (`self.FoodOrder`))
  (if (and (`self.ActorHasTag` OtherActor "food") (`ActorComponent.ComponentHasTag` OtherComp "BaseItemCol") (`self.Enable-end-overlap`))
    (`KismetArrayLibrary.Array_Remove` _foodorder (`KismetArrayLibrary.Array_Find` _foodorder OtherActor))))

(event `/Game/Blueprints/BPI/BPI_GameMode.Clear`
  (set `self.Enable-end-overlap` false)
  (for _array_element (`self.FoodOrder`)
    (`self.K2_DestroyActor` _array_element))
  (`KismetArrayLibrary.Array_Clear` (`self.FoodOrder`))
  (set `self.Enable-end-overlap` true))

(fn `GetWidget`
  (returns (widgetRef :type "/Game/Widgets/TV_Widgets/W_MainOrderScreen Object Reference"))
  (return null))

(fn `HandleReciveFood`
  (returns (FoodOrder :type "Array of Actor Object Reference"))
  (if (> (`KismetArrayLibrary.Array_Length` (`self.FoodOrder`)) 0)
    (return (`self.FoodOrder`))))

(fn `Recive item recipe Tags`
  (returns (Tags :type "GameplayTagContainer Structure"))
  (return))

(fn `UserConstructionScript`)