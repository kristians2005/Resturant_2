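; BP_BaseItem_FoodTray is a kitchen food tray item that acts as a container with a capacity of one.
; On BeginPlay it runs the parent logic, then initializes its BPCContainer component with itself as owner.
; FMInteract passes the currently held item to the container's Examine, delegating interaction handling to that component.
; FlatModeInteraction reports the tray as the target actor along with a fixed interaction type.
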(event `self.ReceiveBeginPlay`
  (`parent.ReceiveBeginPlay`)
  (`/Game/Blueprints/BPC/BPC_Container.Init` (`self.BPC_Container`) self 1 (`self.gup`)))

(event `/Game/Blueprints/BPI/BPI_Interaction.FM_Interact`
  (params (CurrentHoldItem :type "/Game/Blueprints/CookingItems/A_BP_BaseItem_Master Object Reference"))
  (`/Game/Blueprints/BPC/BPC_Container.Examine` (`self.BPC_Container`) CurrentHoldItem))

(fn `FlatMode_Interaction`
  (returns (BaseItemMasterRef :type "/Game/Blueprints/CookingItems/A_BP_BaseItem_Master Object Reference") (InteractionType :type "/Game/Blueprints/Enums/E_InteractionTypes Enum") (Actor :type "Actor Object Reference"))
  (return self "NewEnumerator2" self))

(fn `UserConstructionScript`
  (`parent.UserConstructionScript`))