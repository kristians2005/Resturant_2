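; Spoon kitchen tool for the cooking items, built on a parent item class and holding its own container component.
; BeginPlay initializes that container with the child components of Scene1, a maximum amount and a type.
; Outside flat mode, its Sphere overlapping a component tagged "container" sends a fill-container message to that component's actor.
; For flat mode, an interaction function returns the spoon itself with an interaction type.
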(event `self.ReceiveBeginPlay`
  (`parent.ReceiveBeginPlay`)
  (`/Game/Blueprints/BPC/BPC_Container.Init` (`self.BPC_Container`) self (`SceneComponent.GetChildrenComponents` (`self.Scene1`) false) (`self.Amount Max`) "NewEnumerator1" false false false))

(event `self.Sphere.OnComponentBeginOverlap`
  (params (OverlappedComponent :type "PrimitiveComponent Object Reference") (OtherActor :type "Actor Object Reference") (OtherComp :type "PrimitiveComponent Object Reference") (OtherBodyIndex :type Integer) (bFromSweep :type Boolean) (SweepResult :type "HitResult Structure (by ref)"))
  (if (`/Game/Blueprints/BPFL/BPFL_GlobalFunctions.IsFlatmode`)
    _
    (elif (`KismetArrayLibrary.Array_Contains` (`ActorComponent.ComponentTags` OtherComp) "container")
      (`/Game/Blueprints/BPFL/BPFL_GlobalFunctions.Debug - Print string` (`KismetSystemLibrary.GetDisplayName` OtherActor) false)
      (message `/Game/Blueprints/BPI/BPI_BaseItem.FillContainerr` OtherActor))))

(fn `FlatMode_Interaction`
  (returns (BaseItemMasterRef :type "/Game/Blueprints/CookingItems/A_BP_BaseItem_Master Object Reference") (InteractionType :type "/Game/Blueprints/Enums/E_InteractionTypes Enum") (Actor :type "Actor Object Reference"))
  (return self "NewEnumerator0" self))

(fn `UserConstructionScript`
  (`parent.UserConstructionScript`))