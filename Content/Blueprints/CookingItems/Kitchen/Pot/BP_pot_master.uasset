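; Base Blueprint for kitchen pots among the cooking items, acting as a container that responds to interaction with the player's held item.
; On BeginPlay it initializes its BPCContainer component with itself, a maximum amount and a Gup value.
; FMInteract passes the currently held item to the container's Examine, leaving the handling to that component.
; The flat-mode interaction query returns the pot itself with a fixed interaction type.
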(event `self.ReceiveBeginPlay`
  (`parent.ReceiveBeginPlay`)
  (`/Game/Blueprints/BPC/BPC_Container.Init` (`self.BPC_Container`) self (`self.Amount Max`) (`self.gup`)))

(event `/Game/Blueprints/BPI/BPI_Interaction.FM_Interact`
  (params (CurrentHoldItem :type "/Game/Blueprints/CookingItems/A_BP_BaseItem_Master Object Reference"))
  (`/Game/Blueprints/BPC/BPC_Container.Examine` (`self.BPC_Container`) CurrentHoldItem))

(fn `FlatMode_Interaction`
  (returns (BaseItemMasterRef :type "/Game/Blueprints/CookingItems/A_BP_BaseItem_Master Object Reference") (InteractionType :type "/Game/Blueprints/Enums/E_InteractionTypes Enum") (Actor :type "Actor Object Reference"))
  (return self "NewEnumerator2" self))

(fn `UserConstructionScript`
  (`parent.UserConstructionScript`))