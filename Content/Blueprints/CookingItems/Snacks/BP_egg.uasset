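; BP_egg is a snack cooking item that cracks into two eggshells and a yolk.
; LeftSpawnPoint arms cracking, so a later collision box overlap with an actor not tagged VR_Player can trigger it.
; The overlap also requires the base item's relative location length, not its velocity, to exceed a threshold.
; After a short delay, a DoOnce spawns the pieces at component transforms and destroys the egg.
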(event `self.ReceiveBeginPlay`
  (`parent.ReceiveBeginPlay`))

(event `self.ReceiveTick`
  (params (DeltaSeconds :type "Float (single-precision)"))
  (`parent.ReceiveTick` DeltaSeconds))

(event `self.CollisonOverlapBox.OnComponentBeginOverlap`
  (params (OverlappedComponent :type "PrimitiveComponent Object Reference") (OtherActor :type "Actor Object Reference") (OtherComp :type "PrimitiveComponent Object Reference") (OtherBodyIndex :type Integer) (bFromSweep :type Boolean) (SweepResult :type "HitResult Structure (by ref)"))
  (`/Game/Blueprints/BPFL/BPFL_GlobalFunctions.Debug - Print string` (`KismetSystemLibrary.GetDisplayName` OtherComp) false)
  (if (and (> (`KismetMathLibrary.VSize` (`SceneComponent.RelativeLocation` (`self.BaseItem`))) 800.0) (not (`self.ActorHasTag` OtherActor "VR_Player")) (`self.Can crack?`))
    (`KismetSystemLibrary.Delay` 1.0)
    (`/Engine/EditorBlueprintResources/StandardMacros.DoOnce` false
      (:`Completed`
        (`|SpawnActorFromClass` "/Game/Blueprints/CookingItems/Snacks/BP_eggshell.BP_eggshell_C" (`SceneComponent.K2_GetComponentToWorld` (`self.1`)) "Undefined" "MultiplyWithRoot" null null)
        (`|SpawnActorFromClass` "/Game/Blueprints/CookingItems/Snacks/BP_eggshell.BP_eggshell_C" (`SceneComponent.K2_GetComponentToWorld` (`self.2`)) "Undefined" "MultiplyWithRoot" null null)
        (`|SpawnActorFromClass` "/Game/Blueprints/CookingItems/Snacks/BP_eggYolk.BP_eggYolk_C" (`SceneComponent.K2_GetComponentToWorld` (`self.yolk`)) "Undefined" "MultiplyWithRoot" null null)
        (`self.K2_DestroyActor`)))))

(event `/Game/Blueprints/BPI/BPI_BaseItem.LeftSpawnPoint`
  (set `self.Can crack?` true))

(fn `UserConstructionScript`
  (`parent.UserConstructionScript`))