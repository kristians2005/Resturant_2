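; Item container component for cooking: holds food in pots, bowls and tools like spoons, and moves it between them.
; Init builds tag-keyed slots from hidden meshes, which are revealed and textured as contents arrive.
; Examine routes flatmode or VR interaction into FillContainer, which adds held food or transfers content to or from the held item's container, within amount limits.
; Changing cooked state swaps slot materials to raw, cooked or burnt and disables interaction.
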(event `Init`
  (params (ActorRef :type "/Game/Blueprints/CookingItems/A_BP_BaseItem_Master Object Reference") (`Scene componet array` :type "Array of SceneComponent Object Reference") (AmountMax :type Integer) (Type :type "/Game/Blueprints/Enums/E_ToolType Enum" :default "NewEnumerator0") (`Can be taken out` :type Boolean) (`Can food repeat` :type Boolean) (`Ignore Tags?` :type Boolean))
  (`|ExecutionSequence`
    (:`then_0`
      (set `self.Actor Ref` ActorRef)
      (if (not (== (`KismetArrayLibrary.Array_Length` `Scene componet array`) 0))
        (set `self.Scene Componet Array` `Scene componet array`)
        (set `self.AmountMax` AmountMax)
        (for (_array_element _array_index) (`self.Scene Componet Array`)
          (bind _asmesh_component (cast `MeshComponent` _array_element))
          (`KismetArrayLibrary.Array_Set` (`self.ST_Container-content`) _array_index (make `/Game/Blueprints/Structs/ST_Container` (`|GetArrayItem` (`ActorComponent.ComponentTags` _array_element)) null _asmesh_component) true)
          (`SceneComponent.SetVisibility` _array_element false false))
        (`self.Add baseitem to ST_Container`)
        ; Checks if Item is even a container. this is kind stupid but whatever
        (set `self.Is Initilized?` true)
        (set `self.Type` Type)))
    (:`then_1`
      (set `self.Can Be Taken Out` `Can be taken out`)
      (set `self.Can Food Repeat` `Can food repeat`)
      (set `self.Ignore Tags?` `Ignore Tags?`))))

(event `Examine`
  (params (BaseItem_ref :type "/Game/Blueprints/CookingItems/A_BP_BaseItem_Master Object Reference"))
  ; Check if its Flatmode or VR and interaction heppens
  (if (`self.Can interact`)
    (`/Engine/EditorBlueprintResources/StandardMacros.IsValid` BaseItem_ref
      (:`Is Valid`
        (set `self.Held Actor` BaseItem_ref)
        (if (`/Game/Blueprints/BPFL/BPFL_GlobalFunctions.IsFlatmode`)
          (`self.FillContainer`)
          (else
            (`self.VR_Interaction`))))
      (:`Is Not Valid`
        (`/Game/Blueprints/BPFL/BPFL_GlobalFunctions.Debug - Print string` "BPC_Container, Add Items, ActorRef is not valid" true (struct :`R` 1.0 :`G` 0.087205 :`A` 1.0))))))

(event `FillContainer`
  (bind _content (`self.Content`))
  (bind (_output_tag _output_content) (break `/Game/Blueprints/Structs/ST_Container` (`|GetArrayItem` (`/Game/Blueprints/BPC/BPC_Container.ST_Container-content` (`/Game/Blueprints/CookingItems/A_BP_BaseItem_Master.BPC_Container` (`self.Held Actor`))))))
  (if (not (`/Game/Blueprints/BPC/BPC_Container.Is Initilized?` (`/Game/Blueprints/CookingItems/A_BP_BaseItem_Master.BPC_Container` (`self.Held Actor`))))
    (if (or (not (`KismetSystemLibrary.IsValid` _content)) (== _content (`/Game/Blueprints/CookingItems/A_BP_BaseItem_Master.Item` (`self.Held Actor`))))
      (`self.Add food to container`)
      (`/Game/Blueprints/BPFL/BPFL_GlobalFunctions.Debug - Print string` (`KismetTextLibrary.Conv_TextToString` (`|FormatText` "{item} Container was not init" (`self.Held Actor`))) false (struct :`R` 1.0 :`B` 0.02372 :`A` 1.0))
      (else
        (`/Game/Blueprints/BPFL/BPFL_GlobalFunctions.Debug - Print string` (`KismetTextLibrary.Conv_TextToString` (`|FormatText` "{item} Container content is taken" (`self.Held Actor`))) false (struct :`R` 1.0 :`B` 0.012904 :`A` 1.0))))
    (elif (`KismetSystemLibrary.IsValid` _output_content)
      (`self.Transfer from held items to container`)
      (`/Game/Blueprints/BPFL/BPFL_GlobalFunctions.Debug - Print string` (`KismetTextLibrary.Conv_TextToString` (`|FormatText` "{item} Item transfer content to {c}" (`self.Held Actor`) (`self.Actor Ref`))) false (struct :`R` 1.0 :`B` 0.007402 :`A` 1.0))
      (elif (`KismetArrayLibrary.Array_IsEmpty` (`self.ST_Container-content`))
        (`/Game/Blueprints/BPFL/BPFL_GlobalFunctions.Debug - Print string` (`KismetTextLibrary.Conv_TextToString` (`|FormatText` "{item} Content is empty" (`self.Actor Ref`))) false)
        (else
          (`self.Transfer content form container to held item`)
          (`/Game/Blueprints/BPFL/BPFL_GlobalFunctions.Debug - Print string` (`KismetTextLibrary.Conv_TextToString` (`|FormatText` "{cont} Content to {help}" (`self.Actor Ref`) (`self.Held Actor`))) false (struct :`R` 1.0 :`B` 0.174858 :`A` 1.0)))))))

(event `VR_Interaction`
  (if (not (`/Game/Blueprints/BPC/BPC_Container.Is Initilized?` (`/Game/Blueprints/CookingItems/A_BP_BaseItem_Master.BPC_Container` (`self.Held Actor`))))
    _
    (else
      _))
  (switch `/Game/Blueprints/Enums/E_ToolType` (`/Game/Blueprints/BPC/BPC_Container.Type` (`/Game/Blueprints/CookingItems/A_BP_BaseItem_Master.BPC_Container` (`self.Held Actor`)))
    (:`NewEnumerator0`
      _)
    (:`NewEnumerator1`
      _))
  (`self.FillContainer`))

(event `Add food to container`
  (bind _index (`self.Get index by tag` (`/Game/Blueprints/DataAssets/Items/DA_Item.MeshFoodTag` (`/Game/Blueprints/CookingItems/A_BP_BaseItem_Master.Item` (`self.Held Actor`)))))
  (bind (_contains _struct) (`self.Contains tag` (`/Game/Blueprints/DataAssets/Items/DA_Item.MeshFoodTag` (`/Game/Blueprints/CookingItems/A_BP_BaseItem_Master.Item` (`self.Held Actor`)))))
  (bind (_output_tag _output_content _output_mesh _output_color) (break `/Game/Blueprints/Structs/ST_Container` (`|GetArrayItem` (`self.ST_Container-content`) _index)))
  (bind _raw (`/Game/Blueprints/DataAssets/CookedState/DA_Cooked-state.raw` (`/Game/Blueprints/DataAssets/Items/DA_Item.Texture` (`.Content_12_949F31CF4E5A72DE9ABA38A0E998568F` (break `/Game/Blueprints/Structs/ST_Container` _struct)))))
  ; Add food like cheese, pasta ect, to stuff like pots and pizzaScouse
  (if (> (`self.AmountMax`) (`self.Amount`))
    (if (or (`self.Ignore Tags?`) (`self.Contains tag` (`/Game/Blueprints/DataAssets/Items/DA_Item.MeshFoodTag` (`/Game/Blueprints/CookingItems/A_BP_BaseItem_Master.Item` (`self.Held Actor`)))))
      (if (not (`self.Is content full`))
        (if (not (`self.Contains DA_Item` (`/Game/Blueprints/CookingItems/A_BP_BaseItem_Master.Item` (`self.Held Actor`))))
          (`KismetArrayLibrary.Array_Set` (`self.ST_Container-content`) _index (make `/Game/Blueprints/Structs/ST_Container` _output_tag (`/Game/Blueprints/CookingItems/A_BP_BaseItem_Master.Item` (`self.Held Actor`)) _output_mesh _output_color)))
        (`self.IncreaseAmountt` 1
          (:`Sucsessfuly added`
            (`self.Toggle mesh visibility` (`.Mesh_14_010539C545590258C1B3789506EE96D1` (break `/Game/Blueprints/Structs/ST_Container` (`.Struct` (`self.Contains tag` (`/Game/Blueprints/DataAssets/Items/DA_Item.MeshFoodTag` (`/Game/Blueprints/CookingItems/A_BP_BaseItem_Master.Item` (`self.Held Actor`))))))) true)
            (`/Engine/EditorBlueprintResources/StandardMacros.IsValid` (`.Mesh_14_010539C545590258C1B3789506EE96D1` (break `/Game/Blueprints/Structs/ST_Container` _struct))
              (:`Is Valid`
                (`/Engine/EditorBlueprintResources/StandardMacros.IsValid` _raw
                  (:`Is Valid`
                    (`PrimitiveComponent.SetMaterial` (`.Mesh_14_010539C545590258C1B3789506EE96D1` (break `/Game/Blueprints/Structs/ST_Container` _struct)) 0 _raw)
                    (`self.Debug-Stats` false)))))))))))

(event `Delete held item content`
  (bind _st_container_content (`self.ST_Container-content`))
  (`self.IncreaseAmountt` -1
    (:`Sucsessfuly added`
      (if (== (`self.Amount`) 0)
        (for (_array_element _array_index) (`self.ST_Container-content`)
          (`self.Toggle mesh visibility` (`.Mesh_14_010539C545590258C1B3789506EE96D1` (break `/Game/Blueprints/Structs/ST_Container` _array_element)))
          (bind (_output_tag _output_content _output_mesh _output_color) (break `/Game/Blueprints/Structs/ST_Container` (`|GetArrayItem` _st_container_content _array_index)))
          (`KismetArrayLibrary.Array_Set` _st_container_content 0 (make `/Game/Blueprints/Structs/ST_Container` _output_tag null _output_mesh _output_color)))))))

(event `Transfer from held items to container`
  (bind _st_container_content (`self.ST_Container-content`))
  (bind (_output_tag _output_content _output_mesh) (break `/Game/Blueprints/Structs/ST_Container` (`|GetArrayItem` (`self.ST_Container-content`))))
  (bind (_output_tag_2 _output_content_2 _output_mesh_2 _output_color) (break `/Game/Blueprints/Structs/ST_Container` (`|GetArrayItem` _st_container_content)))
  ; Transfer from Tool like spoon to container like pot, bowl ect
  (if (< (`self.Amount`) (`self.AmountMax`))
    (if (not (`KismetArrayLibrary.Array_IsEmpty` (`/Game/Blueprints/BPC/BPC_Container.ST_Container-content` (`/Game/Blueprints/CookingItems/A_BP_BaseItem_Master.BPC_Container` (`self.Held Actor`)))))
      (`|ExecutionSequence`
        (:`then_0`
          (bind _newparam (message `/Game/Blueprints/BPI/BPI_Container.TransferContentOutput` (`/Game/Blueprints/CookingItems/A_BP_BaseItem_Master.BPC_Container` (`self.Held Actor`))))
          (`KismetArrayLibrary.Array_Set` _st_container_content 0 (make `/Game/Blueprints/Structs/ST_Container` _output_tag_2 (`.Content_12_949F31CF4E5A72DE9ABA38A0E998568F` (break `/Game/Blueprints/Structs/ST_Container` _newparam)) _output_mesh_2 _output_color))
          (`self.Delete held item content` (`/Game/Blueprints/CookingItems/A_BP_BaseItem_Master.BPC_Container` (`self.Held Actor`))))
        (:`then_1`
          (`self.IncreaseAmountt` 1
            (:`Sucsessfuly added`
              (`self.Toggle mesh visibility` _output_mesh true)
              (`PrimitiveComponent.SetMaterial` _output_mesh 0 (`/Game/Blueprints/DataAssets/CookedState/DA_Cooked-state.raw` (`/Game/Blueprints/DataAssets/Items/DA_Item.Texture` _output_content)))
              (`self.Debug-Stats` false))))))))

(event `/Game/Blueprints/BPI/BPI_Container.ChangeMeshCookedState`
  (params (Enum_cooked_state :type "/Game/Blueprints/Enums/E_CookingState Enum" :default "NewEnumerator0"))
  ; Changes the color of Mesh if Cooked state is changed
  (`self.Change item cooked state` Enum_cooked_state))

(event `/Game/Blueprints/BPI/BPI_Container.TransferContainerData`
  (params (`container data` :type "/Game/Blueprints/Structs/ST_Container Structure"))
  (bind _st_container_content (`self.ST_Container-content`))
  (bind (_output_tag _output_content _output_mesh) (break `/Game/Blueprints/Structs/ST_Container` (`|GetArrayItem` _st_container_content)))
  ; Transfer data to from one to other. Example transfer data from held spoon to pot
  (`KismetArrayLibrary.Array_Set` _st_container_content 0 (make `/Game/Blueprints/Structs/ST_Container` _output_tag `container data_Content_12_949F31CF4E5A72DE9ABA38A0E998568F` _output_mesh)))

(event `SetHeldItem`
  (bind (_output_tag _output_content _output_mesh) (break `/Game/Blueprints/Structs/ST_Container` (`|GetArrayItem` (`self.ST_Container-content`))))
  (`self.IncreaseAmountt` 1
    (:`Sucsessfuly added`
      (`self.Toggle mesh visibility` _output_mesh true)
      (`PrimitiveComponent.SetMaterial` _output_mesh 0 (`/Game/Blueprints/DataAssets/CookedState/DA_Cooked-state.raw` (`/Game/Blueprints/DataAssets/Items/DA_Item.Texture` _output_content)))
      (`self.Debug-Stats` false))))

(event `Transfer content form container to held item`
  (bind _st_container_content (`self.ST_Container-content`))
  (bind (_output_tag _output_content _output_mesh _output_color) (break `/Game/Blueprints/Structs/ST_Container` (`|GetArrayItem` _st_container_content)))
  ; Example from bowl to held spoon
  (if (`self.Can Be Taken Out`)
    (if (< 0 (`self.Amount`))
      (`|ExecutionSequence`
        (:`then_0`
          (`self.Transfer content` (`/Game/Blueprints/CookingItems/A_BP_BaseItem_Master.BPC_Container` (`self.Held Actor`)))
          (`self.SetHeldItem` (`/Game/Blueprints/CookingItems/A_BP_BaseItem_Master.BPC_Container` (`self.Held Actor`))))
        (:`then_1`
          (`self.IncreaseAmountt` -1
            (:`Sucsessfuly added`
              (if (== (`self.Amount`) 0)
                (for (_array_element _array_index) (`self.ST_Container-content`)
                  (`self.Toggle mesh visibility` (`.Mesh_14_010539C545590258C1B3789506EE96D1` (break `/Game/Blueprints/Structs/ST_Container` _array_element)))
                  (`KismetArrayLibrary.Array_Set` _st_container_content _array_index (make `/Game/Blueprints/Structs/ST_Container` _output_tag null _output_mesh _output_color)))))))))))

(event `clear content`
  (`KismetArrayLibrary.Array_Clear` (`self.ST_Container-content`)))

(fn `Add baseitem to ST_Container`
  (bind _actor_ref (`self.Actor Ref`))
  (if (not (not (`KismetSystemLibrary.IsValid` (`/Game/Blueprints/DataAssets/Items/DA_Item.Texture` (`/Game/Blueprints/CookingItems/A_BP_BaseItem_Master.Item` (`self.Actor Ref`))))))
    (`KismetArrayLibrary.Array_Add` (`self.ST_Container-content`) (make `/Game/Blueprints/Structs/ST_Container` "None" (`/Game/Blueprints/CookingItems/A_BP_BaseItem_Master.Item` _actor_ref) (`/Game/Blueprints/CookingItems/A_BP_BaseItem_Master.BaseItem` _actor_ref)))))

(fn `Change item cooked state`
  (params (Enum :type "/Game/Blueprints/Enums/E_CookingState Enum" :default "NewEnumerator0"))
  (locals (E_CookedState :type "/Game/Blueprints/Enums/E_CookingState Enum" :default "NewEnumerator0"))
  (set `local.E_CookedState` Enum)
  (set `self.Can interact` false)
  (for _array_element (`self.ST_Container-content`)
    (`/Engine/EditorBlueprintResources/StandardMacros.IsValid` (`.Content_12_949F31CF4E5A72DE9ABA38A0E998568F` (break `/Game/Blueprints/Structs/ST_Container` _array_element))
      (:`Is Valid`
        (bind _texture (`/Game/Blueprints/DataAssets/Items/DA_Item.Texture` (`.Content_12_949F31CF4E5A72DE9ABA38A0E998568F` (break `/Game/Blueprints/Structs/ST_Container` _array_element))))
        (`/Engine/EditorBlueprintResources/StandardMacros.IsValid` _texture
          (:`Is Valid`
            (`PrimitiveComponent.SetMaterial` (`.Mesh_14_010539C545590258C1B3789506EE96D1` (break `/Game/Blueprints/Structs/ST_Container` _array_element)) 0 (select `/Game/Blueprints/Enums/E_CookingState` (`local.E_CookedState`) :`NewEnumerator0` (`/Game/Blueprints/DataAssets/CookedState/DA_Cooked-state.raw` _texture) :`NewEnumerator1` (`/Game/Blueprints/DataAssets/CookedState/DA_Cooked-state.cooked` _texture) :`NewEnumerator2` (`/Game/Blueprints/DataAssets/CookedState/DA_Cooked-state.burnt` _texture)))))))))

(fn `ChangeColor`
  (params (Color :type "LinearColor Structure") (CurrentMesh :type "SceneComponent Object Reference"))
  (locals (MateralRef :type "MaterialInstanceDynamic Object Reference"))
  (set `self.Color` Color)
  (bind _asstatic_mesh_component (cast `StaticMeshComponent` CurrentMesh))
  (bind _returnvalue (`PrimitiveComponent.CreateDynamicMaterialInstance` _asstatic_mesh_component 0 (`PrimitiveComponent.GetMaterial` _asstatic_mesh_component 0) "None"))
  (bind _output_get (set `local.MateralRef` _returnvalue))
  (`MaterialInstanceDynamic.SetVectorParameterValue` _output_get "color" (`self.Color`)))

(fn `Contains DA_Item`
  (params (DA_Item :type "/Game/Blueprints/DataAssets/Items/DA_Item Object Reference"))
  (returns (contains :type Boolean))
  (locals (L_DA_item :type "/Game/Blueprints/DataAssets/Items/DA_Item Object Reference"))
  (set `local.L_DA_item` DA_Item)
  (for _array_element (`self.ST_Container-content`)
    (if (== (`.Content_12_949F31CF4E5A72DE9ABA38A0E998568F` (break `/Game/Blueprints/Structs/ST_Container` _array_element)) (`local.L_DA_item`))
      (return true)))
  (return false))

(fn `Contains tag`
  (params (tag :type Name))
  (returns (Contains :type Boolean) (Struct :type "/Game/Blueprints/Structs/ST_Container Structure"))
  (locals (L_Tag :type Name))
  (set `local.L_Tag` tag)
  (for _array_element (`self.ST_Container-content`)
    (if (== (`.Tag_2_D5A542284C1EE083572AA0A5EE25B82B` (break `/Game/Blueprints/Structs/ST_Container` _array_element)) (`local.L_Tag`))
      (return true _array_element)))
  (return false))

(fn `Debug-Stats`
  (params (bPrintToScreen :type Boolean))
  (`/Game/Blueprints/BPFL/BPFL_GlobalFunctions.Debug - Print string` (`KismetTextLibrary.Conv_TextToString` (`|FormatText` "Amount: {a} \nContainer actor: {c} \nHeld actor {v}" (`self.Amount`) (`self.Actor Ref`) (`self.Held Actor`))) bPrintToScreen)
  (for (_array_element _array_index) (`self.ST_Container-content`)
    (`/Game/Blueprints/BPFL/BPFL_GlobalFunctions.Debug - Print string` (`KismetTextLibrary.Conv_TextToString` (`|FormatText` "index: {1} \ntag: {tag} \ncontent: {2} \nmesh: {3}" _array_index (break `/Game/Blueprints/Structs/ST_Container` _array_element) (`.Content_12_949F31CF4E5A72DE9ABA38A0E998568F` (break `/Game/Blueprints/Structs/ST_Container` _array_element)) (`.Mesh_14_010539C545590258C1B3789506EE96D1` (break `/Game/Blueprints/Structs/ST_Container` _array_element)))) bPrintToScreen (struct :`R` 0.328021 :`G` 0.077846 :`B` 1.0 :`A` 1.0))))

(fn `DecreaseAmount`
  (set `self.Amount` (- (`self.Amount`) 1)))

(fn `Get index by tag`
  (params (tag :type Name))
  (returns (index :type Integer))
  (locals (L_tag :type Name))
  (set `local.L_tag` tag)
  (for (_array_element _array_index) (`self.ST_Container-content`)
    (if (== (`.Tag_2_D5A542284C1EE083572AA0A5EE25B82B` (break `/Game/Blueprints/Structs/ST_Container` _array_element)) (`local.L_tag`))
      (return _array_index)))
  (return 0))

(fn `IncreaseAmount`
  (params (`How much to add?` :type Integer))
  (set `self.Amount` (+ (`self.Amount`) `How much to add?`)))

(fn `Is content full`
  (returns (`is full?` :type Boolean))
  (for _array_element (`self.ST_Container-content`)
    (if (not (`KismetSystemLibrary.IsValid` (`.Content_12_949F31CF4E5A72DE9ABA38A0E998568F` (break `/Game/Blueprints/Structs/ST_Container` _array_element))))
      (return false)))
  (return true))

(fn `Toggle mesh visibility`
  (params (Mesh :type "SceneComponent Object Reference") (`new Visibility` :type Boolean))
  (`/Engine/EditorBlueprintResources/StandardMacros.IsValid` Mesh
    (:`Is Valid`
      (if (`SceneComponent.IsVisible` Mesh)
        (if (not `new Visibility`)
          (`SceneComponent.SetVisibility` Mesh false false))
        (return)
        (else
          (if `new Visibility`
            (`SceneComponent.SetVisibility` Mesh true false))
          (return))))))

(fn `Transfer content`
  (params (`transfer content BPC` :type "Object Object Reference"))
  (for _array_element (`self.ST_Container-content`)
    (message `/Game/Blueprints/BPI/BPI_Container.TransferContainerData` `transfer content BPC` _array_element))
  (return))

(fn `TransferContent`
  (params (Content :type "/Game/Blueprints/DataAssets/Items/DA_Item Object Reference") (`Apply content var` :type Boolean) (InputPin :type "LinearColor Structure") (`Apply color to Gup` :type Boolean))
  (if `Apply content var`
    (set `self.Content` Content)
    (if `Apply color to Gup`
      (bind _output_get (set `self.Color` InputPin))
      (`self.ChangeColor` _output_get))))

(fn `TransferContentOutput`
  (returns (NewParam :type "/Game/Blueprints/Structs/ST_Container Structure"))
  (return (`|GetArrayItem` (`self.ST_Container-content`))))