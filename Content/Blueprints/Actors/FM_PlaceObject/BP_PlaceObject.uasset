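; BP_PlaceObject is a flat-mode interactable spot where the player sets down held items of allowed classes.
; Hovering with a matching item briefly flashes a Niagara effect.
; Interacting has the cached VRPawn place the item at PlaceLocation, then turns off its physics simulation.
; Both actions require an exact class match against AllowedObjects, and the actor reports its interaction type through FlatModeInteraction.
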(event `self.ReceiveBeginPlay`
  (if (`/Game/Blueprints/BPFL/BPFL_GlobalFunctions.IsFlatmode`)
    (bind _asvrpawn (cast `/Game/Game_BP/VRTemplate/Blueprints/VRPawn` (`GameplayStatics.GetPlayerPawn` 0)))
    (set `self.PlayerRef` _asvrpawn)))

(event `/Game/Blueprints/BPI/BPI_Interaction.Hover_Object-snap`
  (params (BP_BaseItem :type "/Game/Blueprints/CookingItems/A_BP_BaseItem_Master Object Reference"))
  (if (`/Game/Blueprints/BPFL/BPFL_GlobalFunctions.IsFlatmode`)
    (if (`SceneComponent.IsVisible` (`self.Niagara`))
      _
      (elif (not (not (`self.Does object match with allowed objects` BP_BaseItem)))
        (`SceneComponent.SetVisibility` (`self.Niagara`) true false)
        (`KismetSystemLibrary.Delay` 0.1)
        (`SceneComponent.SetVisibility` (`self.Niagara`) false false)))))

(event `/Game/Blueprints/BPI/BPI_Interaction.FM_Interact`
  (params (CurrentHoldItem :type "/Game/Blueprints/CookingItems/A_BP_BaseItem_Master Object Reference"))
  (if (`/Game/Blueprints/BPFL/BPFL_GlobalFunctions.IsFlatmode`)
    (set `self.Current Held Object` CurrentHoldItem)
    (if (`KismetArrayLibrary.Array_IsEmpty` (`self.AllowedObjects`))
      _
      (elif (not (not (`self.Does object match with allowed objects` (`self.Current Held Object`))))
        (`/Game/Game_BP/VRTemplate/Blueprints/VRPawn.FM_PlaceItemDown` (`self.PlayerRef`) (`/Game/Blueprints/CookingItems/A_BP_BaseItem_Master.BaseItem` (`self.Current Held Object`)) (`SceneComponent.K2_GetComponentLocation` (`self.PlaceLocation`)) false)
        (`/Game/Blueprints/BPI/BPI_BaseItem.SetSimulatePhisics?` (`self.Current Held Object`) false)))))

(fn `Does object match with allowed objects`
  (params (Object :type "Object Object Reference"))
  (returns (`Does match?` :type Boolean))
  (for _array_element (`self.AllowedObjects`)
    (if (== _array_element (`GameplayStatics.GetObjectClass` Object))
      (return true)))
  (return false))

(fn `FlatMode_Interaction`
  (returns (BaseItemMasterRef :type "/Game/Blueprints/CookingItems/A_BP_BaseItem_Master Object Reference") (InteractionType :type "/Game/Blueprints/Enums/E_InteractionTypes Enum") (Actor :type "Actor Object Reference"))
  (return null "NewEnumerator2" self))

(fn `UserConstructionScript`)