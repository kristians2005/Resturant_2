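; A Blueprint function library of global helpers, mostly for developer debugging, plus queries for developer-code and flatmode flags.
; The flag checks fetch their values from the GameInstance, and the developer-code flag gates the generic string and tag-container debug prints.
; MakeTagKey joins a container's tags into a "+"-separated string key, optionally printing it.
; The anchor-index dump prints each tag and its recipe data assets without that gate.
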(fn `Debug - GameplayTagContainer`
  (params (GPTC :type "GameplayTagContainer Structure") (`GPTC Arr` :type "Array of GameplayTagContainer Structure") (`print?` :type Boolean :default true))
  (locals (`L - Show?` :type Boolean))
  (bind _l___show_ (`local.L - Show?`))
  (set `local.L - Show?` `print?`)
  (if (`self.ShowDeveloperCode` null)
    (if (`KismetArrayLibrary.Array_IsEmpty` `GPTC Arr`)
      (`KismetSystemLibrary.PrintString` null (`BlueprintGameplayTagLibrary.GetDebugStringFromGameplayTagContainer` GPTC) _l___show_ true (struct :`R` 0.39985 :`B` 1.0 :`A` 1.0) 30.0)
      (else
        (for _array_element `GPTC Arr`
          (`KismetSystemLibrary.PrintString` null (`BlueprintGameplayTagLibrary.GetDebugStringFromGameplayTagContainer` _array_element) _l___show_ true (struct :`R` 0.39985 :`B` 1.0 :`A` 1.0) 30.0))))))

(fn `Debug - Print string`
  (params (InString :type String) (bPrintToScreen :type Boolean :default true) (TextColor :type "LinearColor Structure" :default (struct :`R` 0.228885 :`G` 0.337073 :`B` 1.0 :`A` 1.0)) (Duration :type "Float (single-precision)" :default 30.0))
  (if (`self.ShowDeveloperCode` null)
    (`KismetSystemLibrary.PrintString` null InString bPrintToScreen true TextColor Duration)))

(fn `Debug - ST_AnchorIndex`
  (params (AnchorIndex :type "Array of /Game/Blueprints/Structs/ST_AnchorIndex Structure") (bPrintToScreen :type Boolean))
  (locals (`L-Print to screen` :type Boolean))
  (set `local.L-Print to screen` bPrintToScreen)
  (for _array_element AnchorIndex
    (bind (_index _allrecipesvalue) (break `/Game/Blueprints/Structs/ST_AnchorIndex` _array_element))
    (`KismetSystemLibrary.PrintText` null (`|FormatText` "key: {key} {lenght}" (`BlueprintGameplayTagLibrary.GetDebugStringFromGameplayTag` _index) (`KismetArrayLibrary.Array_Length` _allrecipesvalue)) (`local.L-Print to screen`) true (struct :`R` 1.0 :`B` 0.003603 :`A` 1.0) 30.0)
    (for _array_element_2 _allrecipesvalue
      (`KismetSystemLibrary.PrintText` null (`|FormatText` "DataAsset: {key}" (`KismetSystemLibrary.GetDisplayName` _array_element_2)) (`local.L-Print to screen`) true (struct :`R` 1.0 :`G` 0.259932 :`B` 0.136122 :`A` 1.0) 30.0))))

(fn `IsFlatmode`
  (returns (`IsFlatmode?` :type Boolean))
  (bind _isflatmode_ (message `/Game/Blueprints/BPI/BPI_Instance.IsFlatmode` (`GameplayStatics.GetGameInstance` null)))
  (return _isflatmode_))

(fn `MakeTagKey(Tags: GameplayTagContainer) → String`
  (params (GameplayTagContainer :type "GameplayTagContainer Structure (by ref)") (`debug string?` :type Boolean))
  (returns (Tagkeys :type String))
  (locals (`L-AllTags` :type "Array of String"))
  (bind _returnvalue (`KismetStringLibrary.JoinStringArray` (`local.L-AllTags`) "+"))
  (for _array_element (`BlueprintGameplayTagLibrary.BreakGameplayTagContainer` GameplayTagContainer)
    (`KismetArrayLibrary.Array_Add` (`local.L-AllTags`) (`BlueprintGameplayTagLibrary.GetDebugStringFromGameplayTag` _array_element)))
  (`KismetSystemLibrary.PrintString` null _returnvalue `debug string?` true (struct :`G` 0.66 :`B` 1.0 :`A` 1.0) 222.0)
  (return _returnvalue))

(fn `ShowDeveloperCode`
  (returns (ShowDeveloperCode :type Boolean))
  (bind _showdevelopercode (message `/Game/Blueprints/BPI/BPI_Instance.ShowDeveloperCode` (`GameplayStatics.GetGameInstance` null)))
  (return _showdevelopercode))